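; Player controller for a team-based FPS that handles team selection, pawn spawning and the player's UI.
; BeginPlay shows team selection over a level camera; a pick goes through a server event to the GameMode.
; SpawnPlayer spawns and possesses the team's pawn class, then a client event switches to HUD and game input.
; Client events also manage lazily created widgets and win announcements, while Tick formats GameState's remaining time for the HUD timer.
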(event Custom|ShowHideWidget
  (params (Widget :type E_GameWidgets%20Enum :default "NewEnumerator0") (bShow :type Boolean))
  ;[0.25 0.3 1 0.25 24] Shows and hides the widgets.
  (CallFunction|CLShowHideWidget Widget bShow))

(event Custom|CL_ShowHideWidget
  (params (Widget :type E_GameWidgets%20Enum :default "NewEnumerator0") (bShow :type Boolean))
  ;[0.25 0.3 1 0.25 24] Shows and hides the widgets.
  (if bShow
    (CallFunction|FShowWidget Widget)
    (else
      (CallFunction|FHideWidget Widget))))

(event Custom|SpawnPlayer
  (params (Team :type Actor%20Class%20Reference) (SpawnTransform :type Transform))
  ;[0.25 0.3 1 0.25 24] Selects the team and spawns the player
  (bind _returnvalue (Game|SpawnActorfromClass Team SpawnTransform "AdjustIfPossibleButAlwaysSpawn" "MultiplyWithRoot" 0 0))
  (bind _output_get (Variables|References|SetPlayerPawn _returnvalue))
  (bind _player (Class|INTPlayerBase|GetPlayerRef(Message) _output_get))
  (Pawn|Possess _player)
  (CallFunction|CLSpawnPlayer))

(event Custom|SelectTeam
  (params (Team :type Actor%20Class%20Reference))
  ;[0.25 0.3 1 0.25 24] Selects the team and spawns the player
  (CallFunction|SRVSelectTeam Team))

(event Custom|SRV_SelectTeam
  (params (Team :type Actor%20Class%20Reference))
  ;[0.25 0.3 1 0.25 24] Selects the team and spawns the player
  (bind _output_get (Variables|PlayerProperties|SetTeam Team))
  (Default|RequestSpawnPlayer (Variables|References|GetGameMode) self _output_get))

(event Custom|CL_SpawnPlayer
  ;[0.25 0.3 1 0.25 24] Selects the team and spawns the player
  (CallFunction|ShowHideWidget "NewEnumerator0" false)
  (CallFunction|ShowHideWidget "NewEnumerator5" true)
  (CallFunction|ShowHideWidget "NewEnumerator6" true)
  (Input|SetInputModeGameOnly self false)
  (Variables|Default|SetbShowMouseCursor false)
  (Variables|Default|SetbStartMatchTimer true))

(event Custom|UpdateTeamWinAnnouncement
  (params (Team :type Actor%20Class%20Reference) (Score :type Integer) (DisplayTime :type Float%20%28double-precision%29))
  ;[0.25 0.3 1 0.25 24] Updates the Team Announcement UI and displays. Also plays Sound Effect.
  (CallFunction|CLUpdateTeamWinAnnouncement Team Score DisplayTime))

(event Custom|CL_UpdateTeamWinAnnouncement
  (params (Team :type Actor%20Class%20Reference) (Score :type Integer) (DisplayTime :type Float%20%28double-precision%29))
  (bind _wb_main (Variables|WidgetReferences|GetWB_Main))
  ;[0.25 0.3 1 0.25 24] Updates the Team Announcement UI and displays. Also plays Sound Effect.
  (Default|UpdateTeamWinAnnouncementUI (Variables|WidgetReferences|GetWB_Main) Team DisplayTime)
  (if (== Team "/Game/Blueprints/Player/BP_CounterTerrorist.BP_CounterTerrorist_C")
    (Default|UpdateCounterTerroristScoreUI _wb_main Score)
    (else
      (Default|UpdateTerroristScoreUI _wb_main Score)))
  (Audio|PlaySound2D 0 1.0 1.0 0.0 0 0))

(event Custom|TimerCouunter
  (if (Variables|Default|GetbStartMatchTimer)
    (bind _gamestateref (Variables|Default|GetGameStateRef)
      (:then
        (bind _wb_main (Variables|WidgetReferences|GetWB_Main)
          (:then
            (Default|SetTimerText _wb_main (Utilities|Text|FormatText "{Min, number, 00}:{Secs, number, 00} 
" (/ (Variables|/Script/CustomFPS.CustomGameState|GetRemainingTime _gamestateref) 60) (Math|Integer|%(Integer) (Variables|/Script/CustomFPS.CustomGameState|GetRemainingTime _gamestateref) 60))))
          (:else)))
      (:else))))

(event EventTick
  (params (DeltaSeconds :type Float%20%28single-precision%29))
  (CallFunction|TimerCouunter))

(event EventBeginPlay
  ;[0.25 0.3 1 0.25 24] Begin Play
  (CallFunction|ShowHideWidget "NewEnumerator0" true)
  (bind _gamemode (Class|INTGameMode|GetGameModeRef(Message) (Game|GetGameMode)))
  (Variables|References|SetGameMode _gamemode)
  (bind _returnvalue (Actor|GetActorOfClass "/Script/Engine.CameraActor"))
  (Game|Player|SetViewTargetwithBlend _returnvalue 0.0 "VTBlend_Linear" 0.0 false)
  (Input|SetInputModeUIOnly self 0 "DoNotLock" false)
  (Variables|Default|SetbShowMouseCursor true)
  (CallFunction|ShowHideWidget "NewEnumerator7" true)
  (bind _asgs_custom_fps (Utilities|Casting|CastToGS_CustomFPS (Game|GetGameState)))
  (Variables|Default|SetGameStateRef _asgs_custom_fps))

(fn ConstructionScript)

(fn FShowWidget
  (params (Widget :type E_GameWidgets%20Enum :default "NewEnumerator0"))
  (switch Utilities|FlowControl|Switch|SwitchonE_GameWidgets Widget
    (:NewEnumerator5
      (Variables|WidgetReferences|GetWB_Main
        (:then
          _)
        (:else
          (bind _returnvalue (UserInterface|CreateWidget "/Game/UI/Widgets_MainMenu/WB_Main.WB_Main_C"))
          (bind _output_get (Variables|WidgetReferences|SetWB_Main _returnvalue))))
      (UserInterface|Viewport|AddtoViewport _output_get 0))
    (:NewEnumerator0
      (Variables|WidgetReferences|GetWB_TeamSelection
        (:then
          _)
        (:else
          (bind _returnvalue_2 (UserInterface|CreateWidget "/Game/UI/Widgets_MainMenu/WB_TeamSelection.WB_TeamSelection_C"))
          (bind _output_get_2 (Variables|WidgetReferences|SetWB_TeamSelection _returnvalue_2))))
      (UserInterface|Viewport|AddtoViewport _output_get_2 0))
    (:NewEnumerator6
      (Variables|WidgetReferences|GetWB_Crosshair
        (:then
          _)
        (:else
          (bind _returnvalue_3 (UserInterface|CreateWidget "/Game/UI/Widgets_MainMenu/WB_Crosshair.WB_Crosshair_C"))
          (bind _output_get_3 (Variables|WidgetReferences|SetWB_Crosshair _returnvalue_3))))
      (UserInterface|Viewport|AddtoViewport _output_get_3 0))
    (:NewEnumerator7
      (Variables|WidgetReferences|GetWB%20Scoreboard
        (:then
          _)
        (:else
          (bind _returnvalue_4 (UserInterface|CreateWidget "/Game/UI/Widgets_MainMenu/WB_Scoreboard.WB_Scoreboard_C"))
          (bind _output_get_4 (Variables|WidgetReferences|SetWB%20Scoreboard _returnvalue_4))))
      (UserInterface|Viewport|AddtoViewport _output_get_4 0)
      (Widget|SetVisibility (Variables|WidgetReferences|GetWB%20Scoreboard) "Hidden"))))

(fn FHideWidget
  (params (Widget :type E_GameWidgets%20Enum :default "NewEnumerator0"))
  (switch Utilities|FlowControl|Switch|SwitchonE_GameWidgets Widget
    (:NewEnumerator5
      (bind _wb_main (Variables|WidgetReferences|GetWB_Main)
        (:then
          (Widget|RemovefromParent _wb_main))
        (:else)))
    (:NewEnumerator0
      (bind _wb_teamselection (Variables|WidgetReferences|GetWB_TeamSelection)
        (:then
          (Widget|RemovefromParent _wb_teamselection))
        (:else)))
    (:NewEnumerator6
      (bind _wb_crosshair (Variables|WidgetReferences|GetWB_Crosshair)
        (:then
          (Widget|RemovefromParent _wb_crosshair))
        (:else)))))

(fn GetPlayerControllerRef
  (return self))